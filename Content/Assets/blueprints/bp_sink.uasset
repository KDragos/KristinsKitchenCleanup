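; bp_sink is a sink actor that cleans plates and balloons while they overlap it.
; Begin overlap checks for CleanAbleInterface, then casts to bp_plate or bp_balloon and calls CleanMessage.
; End overlap repeats the check and calls StopClean on plates or StopCleanMessage on balloons.
; Despite the interface check, dispatch relies on concrete casts, so other cleanable actors are ignored.
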(event `self.ReceiveActorBeginOverlap`
  (params (OtherActor :type "Actor Object Reference"))
  (if (`KismetSystemLibrary.DoesImplementInterface` OtherActor "/Game/Assets/blueprints/cleanAbleInterface.cleanAbleInterface_C")
    (bind _asbp_plate (cast `/Game/Assets/blueprints/bp_plate` OtherActor)
      (:`then`
        (message `/Game/Assets/blueprints/cleanAbleInterface.clean` _asbp_plate))
      (:`CastFailed`
        (bind _asbp_balloon (cast `/Game/Assets/blueprints/bp_balloon` OtherActor))
        (message `/Game/Assets/blueprints/cleanAbleInterface.clean` _asbp_balloon)))))

(event `self.ReceiveActorEndOverlap`
  (params (OtherActor :type "Actor Object Reference"))
  (if (`KismetSystemLibrary.DoesImplementInterface` OtherActor "/Game/Assets/blueprints/cleanAbleInterface.cleanAbleInterface_C")
    (bind _asbp_plate (cast `/Game/Assets/blueprints/bp_plate` OtherActor)
      (:`then`
        (`/Game/Assets/blueprints/bp_plate.StopClean` _asbp_plate))
      (:`CastFailed`
        (bind _asbp_balloon (cast `/Game/Assets/blueprints/bp_balloon` OtherActor))
        (message `/Game/Assets/blueprints/cleanAbleInterface.StopClean` _asbp_balloon)))))

(fn `UserConstructionScript`)