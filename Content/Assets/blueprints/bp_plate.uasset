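; Dirty plate actor for a VR kitchen game that can be carried, cleaned in a sink for points, or despawned.
; PickUp and DropOff toggle mesh physics and attachment, with physics first enabled after a random startup delay.
; Clean and StopClean control a timer that counts down, then awards score with confetti and sound before destroying the plate.
; The kitchen manager's delegate triggers Despawn, which plays an end-of-cleaning sound and destroys it.
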(event `self.ReceiveBeginPlay`
  ;[1 1 1] Binds the despawn method to the delegate.
  (bind _outactors (`GameplayStatics.GetAllActorsOfClass` "/Game/Assets/blueprints/bp_kitchenManager.bp_kitchenManager_C"))
  (bind _output_get (set `self.kitchenManager` (`KismetArrayLibrary.Array_Get` _outactors)))
  (add `/Game/Assets/blueprints/bp_kitchenManager.DespawnDishes` _output_get (delegate `Despawn`))
  (`KismetSystemLibrary.Delay` (`KismetMathLibrary.RandomFloatInRange` 0.25 2.5))
  (`PrimitiveComponent.SetSimulatePhysics` (`self.plateMesh`) true))

(event `Despawn`
  ;[1 1 1] Binds the despawn method to the delegate.
  (`GameplayStatics.PlaySoundAtLocation` "/Game/Assets/audio/a_endCleaning_Cue.a_endCleaning_Cue" (`SceneComponent.K2_GetComponentLocation` (`self.plateMesh`)))
  (`self.K2_DestroyActor`))

(event `/Game/Assets/blueprints/cleanAbleInterface.StopClean`
  ;[1 1 1] If players take the plate out of the sink, the cleaning timer stops.
  (`KismetSystemLibrary.K2_ClearTimer` null "CleaningPlate")
  (set `self.isAlreadyCleaning` false))

(event `/Game/Assets/blueprints/cleanAbleInterface.clean`
  ;[1 1 1] Starts the cleaning timer on the plate.
  (if (not (`self.isAlreadyCleaning`))
    (`KismetSystemLibrary.K2_SetTimer` null "CleaningPlate" 1.0 (>= (`self.timeRemaining`) 0.0))))

(event `/Game/Assets/blueprints/pickUpAbleInterface.pickUp`
  (params (actorToAttachTo :type "SceneComponent Object Reference"))
  (bind _platemesh (`self.plateMesh`))
  ;[1 1 1] Pickup
  (`PrimitiveComponent.SetSimulatePhysics` _platemesh false)
  (`/Engine/EditorBlueprintResources/StandardMacros.IsValid` _platemesh
    (:`Is Valid`
      (`SceneComponent.K2_AttachToComponent` (`self.K2_GetRootComponent`) actorToAttachTo "None" "KeepWorld" "KeepWorld" "KeepWorld" true))))

(event `/Game/Assets/blueprints/pickUpAbleInterface.dropOff`
  (bind _platemesh (`self.plateMesh`))
  ;[1 1 1] Drop
  (`/Engine/EditorBlueprintResources/StandardMacros.IsValid` _platemesh
    (:`Is Valid`
      (`PrimitiveComponent.SetSimulatePhysics` _platemesh true)
      (`self.K2_DetachFromActor` "KeepWorld" "KeepWorld" "KeepWorld"))))

(fn `CleaningPlate`
  (bind _returnvalue (`SceneComponent.K2_GetComponentLocation` (`self.plateMesh`)))
  (if (`self.isClean`)
    (bind _asmy_vrgame_mode (cast `/Game/MyVRGameMode` (`GameplayStatics.GetGameMode`))
      (:`then`
        (`/Game/MyVRGameMode.IncreaseScore` _asmy_vrgame_mode (`self.ScoreIfCleaned`))
        (`GameplayStatics.SpawnEmitterAtLocation` "/Game/Assets/particles/p_confetti.p_confetti" _returnvalue)
        (`GameplayStatics.PlaySoundAtLocation` "/Game/Assets/audio/a_cleanedDish_Cue.a_cleanedDish_Cue" _returnvalue)
        (`self.K2_DestroyActor`)
        (return))
      (:`CastFailed`
        (return)))
    (else
      (set `self.isAlreadyCleaning` true)
      (bind _result (`/Engine/EditorBlueprintResources/StandardMacros.DecrementFloat` (`self.timeRemaining`))
        (:`  `
          (if (<= _result 0.0)
            (set `self.isClean` true)
            (return)
            (else
              (return))))))))

(fn `UserConstructionScript`)