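; Balloon actor that players can pick up, drop and clean in the sink for score through MyVRGameMode.
; Clean starts a one-second timer that counts TimeRemaining down, then scores and destroys the balloon on a later tick; StopClean clears it.
; Physics starts after a random delay and toggles with pickup and drop.
; The kitchen manager's dispatcher triggers despawn, while the balloon popper binding to Popped is left unconnected.
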(event `self.ReceiveBeginPlay`
  (bind _outactors (`GameplayStatics.GetAllActorsOfClass` "/Game/Assets/blueprints/bp_kitchenManager.bp_kitchenManager_C"))
  (bind _output_get (set `self.kitchenManager` (`KismetArrayLibrary.Array_Get` _outactors)))
  (add `/Game/Assets/blueprints/bp_kitchenManager.DespawnDishes` _output_get (delegate `Despawn`))
  (`KismetSystemLibrary.Delay` (`KismetMathLibrary.RandomFloatInRange` 0.25 2.5))
  (`PrimitiveComponent.SetSimulatePhysics` (`self.balloon_mesh`) true))

(event `Despawn`
  (`GameplayStatics.PlaySoundAtLocation` "/Game/Assets/audio/a_endCleaning_Cue.a_endCleaning_Cue" (`SceneComponent.K2_GetComponentLocation` (`self.balloon_mesh`)))
  (`self.K2_DestroyActor`))

(event `Popped`
  ;[1 1 1] Listen for balloon popper to send message.
  (`GameplayStatics.PlaySoundAtLocation` "/Game/Assets/audio/a_errorCleaning_Cue.a_errorCleaning_Cue" (`SceneComponent.K2_GetComponentLocation` (`self.balloon_mesh`)))
  (`self.K2_DestroyActor`))

(event `/Game/Assets/blueprints/cleanAbleInterface.StopClean`
  ;[1 1 1] If players take the balloon out of the sink, the cleaning timer stops.
  (`KismetSystemLibrary.K2_ClearTimer` null "cleanBalloon")
  (set `self.isAlreadyCleaning` false))

(event `/Game/Assets/blueprints/pickUpAbleInterface.pickUp`
  (params (actorToAttachTo :type "SceneComponent Object Reference"))
  ;[1 1 1] Pickup
  (`PrimitiveComponent.SetSimulatePhysics` (`self.balloon_mesh`) false)
  (`SceneComponent.K2_AttachToComponent` (`self.K2_GetRootComponent`) actorToAttachTo "None" "KeepWorld" "KeepWorld" "KeepWorld" true))

(event `/Game/Assets/blueprints/cleanAbleInterface.clean`
  ;[1 1 1] Starts the cleaning timer on the balloon
  (if (not (`self.isAlreadyCleaning`))
    (`KismetSystemLibrary.K2_SetTimer` null "cleanBalloon" 1.0 (>= (`self.timeRemaining`) 0.0))))

(event `/Game/Assets/blueprints/pickUpAbleInterface.dropOff`
  ;[1 1 1] Drop
  (`PrimitiveComponent.SetSimulatePhysics` (`self.balloon_mesh`) true)
  (`self.K2_DetachFromActor` "KeepWorld" "KeepWorld" "KeepWorld")
  (`PrimitiveComponent.AddImpulse` (`self.balloon_mesh`) (0.0 0.0 50.0) "None" false))

(fn `cleanBalloon`
  (`KismetSystemLibrary.PrintString` "Cleaning a balloon!")
  (if (`self.isClean`)
    (bind _asmy_vrgame_mode (cast `/Game/MyVRGameMode` (`GameplayStatics.GetGameMode`))
      (:`then`
        (`/Game/MyVRGameMode.IncreaseScore` _asmy_vrgame_mode (`self.ScoreIfCleaned`))
        (`GameplayStatics.PlaySoundAtLocation` "/Game/Assets/audio/a_errorCleaning_Cue.a_errorCleaning_Cue" (`SceneComponent.K2_GetComponentLocation` (`self.balloon_mesh`)))
        (`self.K2_DestroyActor`)
        (return))
      (:`CastFailed`
        (return)))
    (else
      (set `self.isAlreadyCleaning` true)
      (bind _result (`/Engine/EditorBlueprintResources/StandardMacros.DecrementFloat` (`self.timeRemaining`))
        (:`  `
          (if (<= _result 0.0)
            (set `self.isClean` true)
            (return)
            (else
              (return))))))))

(fn `UserConstructionScript`)