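; Kitchen manager for a VR dish-cleaning game that runs the timed round started by the game starter's StartGame event.
; A looping one-second timer spawns plates at random points in a box, adds periodic balloons, and passes the countdown to MyVRGameMode.
; At zero it stops spawning and calls for dish despawn; a later start resets the game.
; Sink-avoidance and score-update logic are present but unwired.
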(event `self.ReceiveBeginPlay`
  ;[1 1 1] Sets up listener for the StartGame button.
  (bind _outactors (`GameplayStatics.GetAllActorsOfClass` "/Game/Assets/blueprints/bp_gameStarter.bp_gameStarter_C"))
  (bind _output_get (set `self.gameStarter` (`KismetArrayLibrary.Array_Get` _outactors)))
  (add `/Game/Assets/blueprints/bp_gameStarter.StartGame` _output_get (delegate `SpawnDirtyDishes`)))

(event `SpawnDirtyDishes`
  (if (`self.GameInProgress`)
    ;[1 1 1] If there's a game in progress, and the timer is up, then we'll reset everything.
    (if (<= (`self.GameTimeRemaining`) 0.0)
      (bind _asmy_vrgame_mode (cast `/Game/MyVRGameMode` (`GameplayStatics.GetGameMode`)))
      (`/Game/MyVRGameMode.ResetGame` _asmy_vrgame_mode)
      (set `self.GameTimeRemaining` (`self.MaxGameTime`))
      ;[1 1 1] Core gameplay loop. Spawns plates every second. When timer is up, despawns the plates.
      (set `self.GameInProgress` true :!label _label)
      (`GameplayStatics.PlaySoundAtLocation` "/Game/Assets/audio/a_startCleaning_Cue.a_startCleaning_Cue" (`SceneComponent.K2_GetComponentLocation` (`self.DefaultSceneRoot`)))
      (`KismetSystemLibrary.K2_SetTimer` null "SpawnDirtyDish" 1.0 true)
      (if (<= (`self.GameTimeRemaining`) 0.0)
        (`self.DespawnDishes`)))
    (else
      (goto _label))))

(fn `GetRandomSpawnPoint`
  (returns (ReturnValue :type "Vector Structure"))
  (return (`KismetMathLibrary.RandomPointInBoundingBox` (`SceneComponent.K2_GetComponentLocation` (`self.DefaultSceneRoot`)) (`self.BoxExtent`))))

(fn `SpawnDirtyDish`
  (locals (NewLocalVar_0 :type "/Game/Assets/blueprints/bp_plate Object Reference"))
  (bind _gametimeremaining (`self.GameTimeRemaining`))
  (`KismetSystemLibrary.PrintString` "Spawning dish!")
  (bind _returnvalue (`self.GetRandomSpawnPoint`))
  (bind _output_get (set `self.spawnPoint` (`KismetMathLibrary.MakeTransform` _returnvalue))) ; Gets a new spawn point.
  (`|SpawnActorFromClass` "/Game/Assets/blueprints/bp_plate.bp_plate_C" _output_get "AdjustIfPossibleButAlwaysSpawn" "OverrideRootScale")
  (if (== (mod _gametimeremaining 5.0) 0.0)
    (bind _returnvalue_2 (`self.GetRandomSpawnPoint`))
    (`|SpawnActorFromClass` "/Game/Assets/blueprints/bp_balloon.bp_balloon_C" (`KismetMathLibrary.MakeTransform` _returnvalue_2 (struct) (0.4 0.4 0.4)) "AdjustIfPossibleButAlwaysSpawn" "OverrideRootScale"))
  (bind _result (`/Engine/EditorBlueprintResources/StandardMacros.DecrementFloat` _gametimeremaining)
    (:`  `
      (bind _asmy_vrgame_mode (cast `/Game/MyVRGameMode` (`GameplayStatics.GetGameMode`)))
      (bind _percentagetimeremaining (`/Game/MyVRGameMode.GetTimeRemaining` _asmy_vrgame_mode _result (`self.MaxGameTime`)))
      (if (<= _gametimeremaining 0.0)
        (`GameplayStatics.PlaySoundAtLocation` "/Game/Assets/audio/a_endCleaning_Cue.a_endCleaning_Cue" (`SceneComponent.K2_GetComponentLocation` (`self.DefaultSceneRoot`)))
        (`KismetSystemLibrary.K2_ClearTimer` null "SpawnDirtyDish")
        (`self.DespawnDishes`)
        (else
          (`KismetSystemLibrary.PrintString` (`KismetStringLibrary.BuildString_Double` "" "Time remaining is: " _percentagetimeremaining)))))))

(fn `UpdateGameScore`)

(fn `UserConstructionScript`)